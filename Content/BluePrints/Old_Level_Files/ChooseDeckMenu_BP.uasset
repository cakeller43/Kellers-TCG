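; Deck selection menu actor with three clickable decks that sends the player's choice to the match player controller.
; Each click sets DeckChoice, calls ChooseDeck on PlayerControllerMatch, then a timeline lerps this menu back to its construction-time transform.
; When that finishes, a second timeline lerps MatchMenu to a fixed end transform, with that menu's input disabled until the move completes.
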(event OnClicked(Deck1)
  (params (TouchedComponent :type Primitive%20Component%20Object%20Reference))
  (bind _matchmenu (Variables|Default|GetMatchMenu))
  (Variables|Default|SetDeckChoice 1)
  (bind _asplayer_controller_match (Utilities|Casting|CastToPlayerControllerMatch (Game|GetPlayerController 0)))
  (Class|PlayerControllerMatch|ChooseDeck _asplayer_controller_match (Variables|Default|GetDeckChoice))
  (bind _newtrack_0 (Timeline|Move%20Menu PlayFromStart)
    (:Update
      (Transformation|SetActorTransform (Math|Transform|Lerp(Transform) (Transformation|GetActorTransform) (Variables|Default|GetStart%20Transform) _newtrack_0)))
    (:Finished
      (Input|DisableInput (Variables|Default|GetMatchMenu) 0)
      (bind _newtrack_0_2 (Timeline|MoveMenu2 PlayFromStart)
        (:Update
          (Transformation|SetActorTransform _matchmenu (Math|Transform|Lerp(Transform) (Transformation|GetActorTransform _matchmenu) (Variables|Default|GetEnd%20Transform) _newtrack_0_2)))
        (:Finished
          (Input|EnableInput _matchmenu 0))))))

(event OnClicked(Deck2)
  (params (TouchedComponent :type Primitive%20Component%20Object%20Reference))
  (bind _matchmenu (Variables|Default|GetMatchMenu))
  (Variables|Default|SetDeckChoice 2)
  (bind _asplayer_controller_match (Utilities|Casting|CastToPlayerControllerMatch (Game|GetPlayerController 0)))
  (Class|PlayerControllerMatch|ChooseDeck _asplayer_controller_match (Variables|Default|GetDeckChoice))
  (bind _newtrack_0 (Timeline|Move%20Menu PlayFromStart)
    (:Update
      (Transformation|SetActorTransform (Math|Transform|Lerp(Transform) (Transformation|GetActorTransform) (Variables|Default|GetStart%20Transform) _newtrack_0)))
    (:Finished
      (Input|DisableInput (Variables|Default|GetMatchMenu) 0)
      (bind _newtrack_0_2 (Timeline|MoveMenu2 PlayFromStart)
        (:Update
          (Transformation|SetActorTransform _matchmenu (Math|Transform|Lerp(Transform) (Transformation|GetActorTransform _matchmenu) (Variables|Default|GetEnd%20Transform) _newtrack_0_2)))
        (:Finished
          (Input|EnableInput _matchmenu 0))))))

(event OnClicked(Deck3)
  (params (TouchedComponent :type Primitive%20Component%20Object%20Reference))
  (bind _matchmenu (Variables|Default|GetMatchMenu))
  (Variables|Default|SetDeckChoice 3)
  (bind _asplayer_controller_match (Utilities|Casting|CastToPlayerControllerMatch (Game|GetPlayerController 0)))
  (Class|PlayerControllerMatch|ChooseDeck _asplayer_controller_match (Variables|Default|GetDeckChoice))
  (bind _newtrack_0 (Timeline|Move%20Menu PlayFromStart)
    (:Update
      (Transformation|SetActorTransform (Math|Transform|Lerp(Transform) (Transformation|GetActorTransform) (Variables|Default|GetStart%20Transform) _newtrack_0)))
    (:Finished
      (Input|DisableInput (Variables|Default|GetMatchMenu) 0)
      (bind _newtrack_0_2 (Timeline|MoveMenu2 PlayFromStart)
        (:Update
          (Transformation|SetActorTransform _matchmenu (Math|Transform|Lerp(Transform) (Transformation|GetActorTransform _matchmenu) (Variables|Default|GetEnd%20Transform) _newtrack_0_2)))
        (:Finished
          (Input|EnableInput _matchmenu 0))))))

(event EventBeginPlay)

(fn ConstructionScript
  (Variables|Default|SetStart%20Transform (Transformation|GetActorTransform))
  (Variables|Default|SetEnd%20transform (Math|Transform|MakeTransform "0.000000,0.000000,100.000000" "0.000000,0.000000, 0")))