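; Game mode that sets up each player on login in a game with two groups of player starts.
; On the server, PostLogin sorts every PlayerStart into Player1 or Player2 arrays by its tag, with any tag other than "Player1" going to Player2.
; It then derives PlayerNumber from the PlayerArray length to keep scoreboard order identical for all players, and calls ClientPostLogin after casting the new controller.
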(event EventPostLogin
  (params (NewPlayer :type Player%20Controller%20Object%20Reference))
  ;[1 1 1] Post login
  (Networking|SwitchHasAuthority
    (:Authority
      (bind _outactors (Actor|GetAllActorsOfClass "/Script/Engine.PlayerStart"))
      (for _array_element _outactors
        (if (Utilities|Name|Equal(Name) (Variables|/Script/Engine.PlayerStart|GetPlayerStartTag _array_element) "Player1")
          (Utilities|Array|AddUnique (Variables|Default|GetPlayer1) _array_element)
          (else
            (Utilities|Array|AddUnique (Variables|Default|GetPlayer2) _array_element))))
      (Utilities|Casting|CastTo (Variables|/Script/Engine.Controller|GetPlayerState NewPlayer))
      (Variables|Default|SetPlayerNumber (Utilities|Array|Length (Variables|/Script/Engine.GameState|GetPlayerArray (Game|GetGameState)))) ; Makes the scoreboard in the same order for all players
      (Utilities|Casting|CastTo NewPlayer)
      (CallFunction|ClientPostLogin))))

(fn ConstructionScript)