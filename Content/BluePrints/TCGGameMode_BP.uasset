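; TCGGameMode_BP is a game mode that sets up each player on login to a match.
; On authority, PostLogin sorts PlayerStart actors into Player1 and Player2 arrays, sending any tag other than "Player1" to Player2.
; It then sets the new MyPlayerState's PlayerNumber from the current PlayerArray length and calls ClientPostLogin on the PlayerControllerMatch_BP.
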(event EventPostLogin
  (params (NewPlayer :type Player%20Controller%20Object%20Reference))
  ;[1 1 1] Post login
  (Networking|SwitchHasAuthority
    (:Authority
      (bind _outactors (Actor|GetAllActorsOfClass "/Script/Engine.PlayerStart"))
      (for _array_element _outactors
        (if (Utilities|Name|Equal(Name) (Variables|/Script/Engine.PlayerStart|GetPlayerStartTag _array_element) "Player1")
          (Utilities|Array|AddUnique (Variables|Default|GetPlayer1) _array_element)
          (else
            (Utilities|Array|AddUnique (Variables|Default|GetPlayer2) _array_element))))
      (bind _asmy_player_state (Utilities|Casting|CastToMyPlayerState (Variables|/Script/Engine.Controller|GetPlayerState NewPlayer)))
      (Variables|/Game/Blueprints/MyPlayerState.MyPlayerState_C|SetPlayerNumber _asmy_player_state (Utilities|Array|Length (Variables|/Script/Engine.GameState|GetPlayerArray (Game|GetGameState))))
      (bind _asplayer_controller_match_bp (Utilities|Casting|CastToPlayerControllerMatch_BP NewPlayer))
      (Default|ClientPostLogin _asplayer_controller_match_bp))))

(fn ConstructionScript)