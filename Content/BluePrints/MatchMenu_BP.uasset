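; MatchMenu_BP is a match menu actor in a card game, with buttons for starting a match, choosing a deck and returning to the Main level.
; Choose Deck uses chained timelines to lerp this menu to a fixed end transform, then DeckSelectionMenu into its original place, disabling that menu's input during the slide.
; The construction script sets both transforms.
; Start Match is empty; a timeline that would initialize TCGGameMode's match state stack is unconnected.
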(event OnClicked(Btn_StartMatch)
  (params (TouchedComponent :type Primitive%20Component%20Object%20Reference)))

(event OnClicked(Btn_ChooseDeck)
  (params (TouchedComponent :type Primitive%20Component%20Object%20Reference))
  (bind _deckselectionmenu (Variables|Default|GetDeckSelectionMenu))
  (bind _newtrack_0 (Timeline|Move%20Menu PlayFromStart)
    (:Update
      (Transformation|SetActorTransform (Math|Transform|Lerp(Transform) (Variables|Default|GetStart%20Transform) (Variables|Default|GetEnd%20Transform) _newtrack_0)))
    (:Finished
      (Input|DisableInput (Variables|Default|GetDeckSelectionMenu) 0)
      (bind _newtrack_0_2 (Timeline|MoveMenu2 PlayFromStart)
        (:Update
          (Transformation|SetActorTransform _deckselectionmenu (Math|Transform|Lerp(Transform) (Transformation|GetActorTransform _deckselectionmenu) (Variables|Default|GetStart%20Transform) _newtrack_0_2)))
        (:Finished
          (Input|EnableInput _deckselectionmenu 0))))))

(event OnClicked(Btn_BackToMain)
  (params (TouchedComponent :type Primitive%20Component%20Object%20Reference))
  (Game|OpenLevel(byName) "Main"))

(event EventBeginPlay)

(fn ConstructionScript
  (Variables|Default|SetStart%20Transform (Transformation|GetActorTransform))
  (Variables|Default|SetEnd%20transform (Math|Transform|MakeTransform "-2000.000000,0.000000,340.000000" "0.000000,-90.000000, 0")))